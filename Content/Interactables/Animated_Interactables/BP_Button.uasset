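; BP_Button is a color-coded pressure button that unlocks a linked TargetDoor.
; The construction script tints the button with PickupColor through a dynamic material instance.
; Overlap by a BP_PhysicsPickup of matching color sets the door's IsUnlocked and plays a timeline lowering the button, or prints a warning if no door is linked.
; Any pickup leaving relocks the door and reverses the timeline, without checking color or door validity.
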(event OnComponentBeginOverlap(overlap)
  (params (OverlappedComponent :type Primitive%20Component%20Object%20Reference) (OtherActor :type Actor%20Object%20Reference) (OtherComp :type Primitive%20Component%20Object%20Reference) (OtherBodyIndex :type Integer) (bFromSweep :type Boolean) (SweepResult :type Hit%20Result%20Structure%20%28by%20ref%29))
  (bind _targetdoor (Variables|Default|GetTargetDoor))
  (bind _asbp_physics_pickup (Utilities|Casting|CastToBP_PhysicsPickup OtherActor))
  (if (== (Variables|/Game/Interactables/BP_PhysicsPickup.BP_PhysicsPickup_C|GetpickupColor _asbp_physics_pickup) (Variables|Default|GetpickupColor))
    (Utilities|IsValid _targetdoor
      (:Is%20Valid
        (Variables|/Game/Interactables/Animated_Interactables/BP_Door.BP_Door_C|SetisUnlocked _targetdoor true)
        (bind _alphatrack (Timeline|alpha Play)
          (:Update
            (Transformation|SetRelativeLocation (Variables|Default|Getbutton) (Math|Vector|MakeVector 0.0 0.0 (Math|Float|Lerp 5.0 1.0 _alphatrack)) false false))))
      (:Is%20Not%20Valid
        (Development|PrintString "forgot to link door")))))

(event OnComponentEndOverlap(overlap)
  (params (OverlappedComponent :type Primitive%20Component%20Object%20Reference) (OtherActor :type Actor%20Object%20Reference) (OtherComp :type Primitive%20Component%20Object%20Reference) (OtherBodyIndex :type Integer))
  (Utilities|Casting|CastToBP_PhysicsPickup OtherActor)
  (Variables|/Game/Interactables/Animated_Interactables/BP_Door.BP_Door_C|SetisUnlocked (Variables|Default|GetTargetDoor) false)
  (bind _alphatrack (Timeline|alpha Reverse)
    (:Update
      (Transformation|SetRelativeLocation (Variables|Default|Getbutton) (Math|Vector|MakeVector 0.0 0.0 (Math|Float|Lerp 5.0 1.0 _alphatrack)) false false))))

(event EventBeginPlay)

(event Collision|EventActorBeginOverlap
  (params (OtherActor :type Actor%20Object%20Reference)))

(event EventTick
  (params (DeltaSeconds :type Float%20%28single-precision%29)))

(fn ConstructionScript
  (bind _returnvalue (Rendering|Material|CreateDynamicMaterialInstance (Variables|Default|Getbutton) 0 "/Game/Interactables/Animated_Interactables/MAT_Color.MAT_Color" "None" :!class /Script/Engine.PrimitiveComponent))
  (bind _output_get (Variables|Default|SetcolorDMI _returnvalue))
  (Rendering|Material|SetVectorParameterValue _output_get "color" (Variables|Default|GetpickupColor) :!class /Script/Engine.MaterialInstanceDynamic))